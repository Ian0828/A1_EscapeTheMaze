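; Floor or wall button actor that opens a linked door for a limited time when the ThirdPersonCharacter overlaps its collision box.
; A timeline animates the Hinge between the Off and On transforms, while debug messages report the press and countdown.
; The door calls hang off the timeline's Update, so OpenDoor repeats during playback.
; CloseDoor follows a ClosingDelay wait, independent of the hardcoded eight-second message.
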(event OnComponentBeginOverlap(BoxCollision)
  (params (OverlappedComponent :type Primitive%20Component%20Object%20Reference) (OtherActor :type Actor%20Object%20Reference) (OtherComp :type Primitive%20Component%20Object%20Reference) (OtherBodyIndex :type Integer) (bFromSweep :type Boolean) (SweepResult :type Hit%20Result%20Structure%20%28by%20ref%29))
  (bind _door (Variables|Default|GetDoor))
  (Utilities|Casting|CastToThirdPersonCharacter OtherActor)
  (Development|PrintString "Botton Pushed")
  (Development|PrintString "Door Opened")
  (Development|PrintString "You have 8 seconds")
  (bind _pressvalue (Timeline|Timeline_0 Play)
    (:Update
      (Transformation|SetRelativeTransform (Variables|Default|GetHinge) (Math|Transform|Lerp(Transform) (Transformation|GetRelativeTransform (Variables|Default|GetOff)) (Transformation|GetRelativeTransform (Variables|Default|GetOn)) _pressvalue) false false)
      (Default|OpenDoor _door)
      (Utilities|FlowControl|Delay (Variables|Default|GetClosingDelay))
      (Default|CloseDoor _door)
      (Development|PrintString "Door Closed"))))

(event EventBeginPlay)

(event Collision|EventActorBeginOverlap
  (params (OtherActor :type Actor%20Object%20Reference)))

(event EventTick
  (params (DeltaSeconds :type Float%20%28single-precision%29)))

(fn ConstructionScript)