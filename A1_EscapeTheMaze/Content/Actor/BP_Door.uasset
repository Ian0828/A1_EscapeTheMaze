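; BP_Door is a door actor that opens and closes through its OpenDoor and CloseDoor events.
; A timeline lerps the Hinge's relative transform between the Close and Open components' transforms, so those components define both poses.
; OpenDoor plays the timeline and CloseDoor reverses it, each setting its own play rate and updating IsOpen.
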(event Custom|OpenDoor
  (Components|Timeline|SetPlayRate (Variables|Default|GetTimeline_0) (Variables|Default|GetOpeningSpeed))
  (Variables|Default|SetIsOpen true)
  (bind _movevalue (Timeline|Timeline_0 Play)
    (:Update
      (Transformation|SetRelativeTransform (Variables|Default|GetHinge) (Math|Transform|Lerp(Transform) (Transformation|GetRelativeTransform (Variables|Default|GetClose)) (Transformation|GetRelativeTransform (Variables|Default|GetOpen)) _movevalue) false false))))

(event Custom|CloseDoor
  (Components|Timeline|SetPlayRate (Variables|Default|GetTimeline_0) (Variables|Default|GetClosingSpeed))
  (Variables|Default|SetIsOpen false)
  (bind _movevalue (Timeline|Timeline_0 Reverse)
    (:Update
      (Transformation|SetRelativeTransform (Variables|Default|GetHinge) (Math|Transform|Lerp(Transform) (Transformation|GetRelativeTransform (Variables|Default|GetClose)) (Transformation|GetRelativeTransform (Variables|Default|GetOpen)) _movevalue) false false))))

(event Collision|EventActorBeginOverlap
  (params (OtherActor :type Actor%20Object%20Reference)))

(event EventTick
  (params (DeltaSeconds :type Float%20%28single-precision%29)))

(fn ConstructionScript)