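; BP_PuzzleTrigger is a trigger actor that opens a door for a player character with the required puzzle progress.
; When a ThirdPersonCharacter enters its BoxCollision, it checks that character's PuzzleCount and opens the referenced Door only if the count is exactly three.
; When any ThirdPersonCharacter leaves the box, it closes the Door regardless of count.
; Both door actions print a debug message.
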(event OnComponentBeginOverlap(BoxCollision)
  (params (OverlappedComponent :type Primitive%20Component%20Object%20Reference) (OtherActor :type Actor%20Object%20Reference) (OtherComp :type Primitive%20Component%20Object%20Reference) (OtherBodyIndex :type Integer) (bFromSweep :type Boolean) (SweepResult :type Hit%20Result%20Structure%20%28by%20ref%29))
  (bind _asthird_person_character (Utilities|Casting|CastToThirdPersonCharacter OtherActor))
  (Math|Integer|CompareInt (Variables|/Game/ThirdPersonBP/Blueprints/ThirdPersonCharacter.ThirdPersonCharacter_C|GetPuzzleCount _asthird_person_character) 3
    (:==
      (if true
        (Default|OpenDoor (Variables|Default|GetDoor))
        (Development|PrintString "Door Opened")))))

(event OnComponentEndOverlap(BoxCollision)
  (params (OverlappedComponent :type Primitive%20Component%20Object%20Reference) (OtherActor :type Actor%20Object%20Reference) (OtherComp :type Primitive%20Component%20Object%20Reference) (OtherBodyIndex :type Integer))
  (Utilities|Casting|CastToThirdPersonCharacter OtherActor)
  (Default|CloseDoor (Variables|Default|GetDoor))
  (Development|PrintString "Door Closed"))

(event EventBeginPlay)

(event Collision|EventActorBeginOverlap
  (params (OtherActor :type Actor%20Object%20Reference)))

(event EventTick
  (params (DeltaSeconds :type Float%20%28single-precision%29)))

(fn ConstructionScript)